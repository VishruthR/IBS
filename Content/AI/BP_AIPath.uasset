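; BP_AIPath is a spline-based path actor that supplies AI with target locations along its route.
; GetClosestLocationToAIPath finds the spline distance nearest the AI's location, adds a look-ahead distance and returns that world position.
; Overshoot past the spline's end wraps by subtracting its length once, treating the path as a loop.
; The event graph and construction script contain no active logic.
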(event EventBeginPlay)

(event Collision|EventActorBeginOverlap
  (params (OtherActor :type Actor%20Object%20Reference)))

(event EventTick
  (params (DeltaSeconds :type Float%20%28single-precision%29)))

(fn ConstructionScript)

(fn GetClosestLocationtoAIPath
  (params (AILocation :type Vector :default "0, 0, 0") (AdditionalDistance :type Float%20%28double-precision%29))
  (bind _spline (Variables|Default|GetSpline))
  (bind _returnvalue (Class|SplineComponent|GetDistanceAlongSplineatLocation _spline AILocation "World"))
  (bind _returnvalue_2 (+ _returnvalue AdditionalDistance))
  (return (Spline|GetLocationatDistanceAlongSpline (Variables|Default|GetSpline) (Math|Float|SelectFloat (- _returnvalue_2 (Spline|GetSplineLength (Variables|Default|GetSpline))) _returnvalue_2 (> _returnvalue_2 (Spline|GetSplineLength (Variables|Default|GetSpline)))) "World")))