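; Bullet is a projectile actor that flies along its Direction until it hits something or its lifetime runs out.
; Tick counts TimeToLive down by delta seconds, destroys the actor at zero, and otherwise moves it a fixed swept step per frame, not scaled by frame time.
; An overlap with any actor other than a BP_SportsCar_Pawn destroys it; no damage is applied here.
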(event Collision|EventActorBeginOverlap
  (params (OtherActor :type Actor%20Object%20Reference))
  (Utilities|Casting|CastToBP_SportsCar_Pawn OtherActor
    (:CastFailed
      (Actor|DestroyActor))))

(event EventTick
  (params (DeltaSeconds :type Float%20%28single-precision%29))
  ;[1 1 1] Bullet shooting logic
  (bind _output_get (Variables|Default|SetTimeToLive (- (Variables|Default|GetTimeToLive) DeltaSeconds)))
  (if (<= _output_get 0.0)
    (Actor|DestroyActor)
    (else
      (Transformation|SetActorTransform (Math|Transform|MakeTransform (+ (* (Variables|Default|GetDirection) "120.000000,120.000000,120.000000") (Transformation|GetActorLocation)) "0, 0, 0" "1.000000,1.000000,1.000000") true))))

(fn ConstructionScript)