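; BP_SpeedPowerUp is an actor that spawns a single BP_Beholder when play begins; despite its name, it contains no speed boost logic.
; The spawn point is random in X and Y within the Cube component's local bounds offset by the actor's location, ignoring component scale and rotation.
; The Beholder spawns at a fixed world height with an enlarged scale.
; Overlap, Tick and the construction script are empty.
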(event EventBeginPlay
  (bind _returnvalue (Transformation|GetActorLocation))
  (bind _cube (Variables|Default|GetCube))
  (bind (_min _max) (Components|StaticMesh|GetLocalBounds _cube))
  (Game|SpawnActorfromClass "/Game/Blueprints/BP_Beholder.BP_Beholder_C" (Math|Transform|MakeTransform (Math|Vector|MakeVector (Math|Random|RandomFloatinRange (+ (.x _min) (.x _returnvalue)) (+ (.x _max) (.x _returnvalue))) (Math|Random|RandomFloatinRange (+ (.y _min) (.y _returnvalue)) (+ (.y _max) (.y _returnvalue))) 1e+02) "0, 0, 0" "1.500000,1.500000,1.500000") "Undefined" "MultiplyWithRoot" 0 0))

(event Collision|EventActorBeginOverlap
  (params (OtherActor :type Actor%20Object%20Reference)))

(event EventTick
  (params (DeltaSeconds :type Float%20%28single-precision%29)))

(fn ConstructionScript)