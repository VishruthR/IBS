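; BP_Pedestrian is a pedestrian pawn that walks back and forth between two target points.
; BeginPlay starts the Roam event, which chains AI MoveTo calls to TargetPoint1 and then TargetPoint2, with a short pause after each arrival, and then calls itself to loop.
; Only successful moves continue the chain, so a failed move stops the patrol.
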(event Custom|Roam
  (AI|AIMoveTo self "0, 0, 0" (Variables|Default|GetTargetPoint1) 1.0 false
    (:OnSuccess
      (Utilities|FlowControl|Delay 0.2)
      (AI|AIMoveTo self "0, 0, 0" (Variables|Default|GetTargetPoint2) 1.0 false
        (:OnSuccess
          (Utilities|FlowControl|Delay 0.2)
          (CallFunction|Roam))))))

(event EventBeginPlay
  (CallFunction|Roam))

(event Collision|EventActorBeginOverlap
  (params (OtherActor :type Actor%20Object%20Reference)))

(event EventTick
  (params (DeltaSeconds :type Float%20%28single-precision%29)))

(fn ConstructionScript)